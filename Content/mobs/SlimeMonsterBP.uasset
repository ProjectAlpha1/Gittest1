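; Slime enemy Blueprint that patrols between TP_4 and TP_3 actors and chases the player on sight or when first hit.
; A Gate cycles two Timelines that lerp the mesh's height, roll and scale into a procedural hop.
; Sphere overlaps apply fireball damage, destroying the slime with a particle effect at zero health.
; Player contact briefly halts movement as a cooldown and toggles IsAttacking, a placeholder for a future attack animation.
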(event `self.ReceiveBeginPlay`
  (bind _height (`self.Height`))
  (bind _slimemonster_final2 (`self.SlimeMonster_Final2`))
  (bind _returnvalue (`SceneComponent.K2_GetComponentRotation` _slimemonster_final2))
  (bind _returnvalue_2 (`SceneComponent.K2_GetComponentRotation` _slimemonster_final2))
  (bind _returnvalue_3 (`SceneComponent.K2_GetComponentLocation` _slimemonster_final2))
  (bind _returnvalue_4 (`SceneComponent.K2_GetComponentScale` _slimemonster_final2))
  (bind _returnvalue_5 (`SceneComponent.K2_GetComponentScale` _slimemonster_final2))
  (bind _returnvalue_6 (`SceneComponent.K2_GetComponentLocation` _slimemonster_final2))
  (`|ExecutionSequence`
    (:`then_0`
      (goto _label :!via `Open`))
    (:`then_1`
      (`/Engine/EditorBlueprintResources/StandardMacros.Gate` true :!label _label
        (:`Exit`
          (bind (_direction _animation_time_frame) (`Timeline|Timeline_0` :!via `PlayFromStart`)
            (:`Update`
              (`SceneComponent.K2_SetWorldLocationAndRotation` _slimemonster_final2 (`KismetMathLibrary.VLerp` _returnvalue_6 (`KismetMathLibrary.MakeVector` (.x _returnvalue_6) (.y _returnvalue_6) (+ (.z _returnvalue_6) _height)) _animation_time_frame) (`KismetMathLibrary.RLerp` _returnvalue_2 (`KismetMathLibrary.MakeRotator` (- (.roll _returnvalue_2) (`self.Rotation`)) (.pitch _returnvalue_2) (.yaw _returnvalue_2)) _animation_time_frame) false false))
            (:`Finished`
              (if (`self.Finished?`)
                (`SceneComponent.SetWorldScale3D` _slimemonster_final2 (`KismetMathLibrary.VLerp` _returnvalue_4 (`KismetMathLibrary.MakeVector` (.x _returnvalue_4) (.y _returnvalue_4) (+ (.z _returnvalue_4) (`self.scale`))) (`self.Alpha`)))
                (bind (_direction_2 _animation_time_frame_2) (`Timeline|Timeline_1` :!via `PlayFromStart` :!label _label_2)
                  (:`Update`
                    (`SceneComponent.K2_SetWorldLocationAndRotation` _slimemonster_final2 (`KismetMathLibrary.VLerp` _returnvalue_3 (`KismetMathLibrary.MakeVector` (.x _returnvalue_3) (.y _returnvalue_3) (- (.z _returnvalue_3) _height)) _animation_time_frame_2) (`KismetMathLibrary.RLerp` _returnvalue (`KismetMathLibrary.MakeRotator` (+ (.roll _returnvalue) (`self.Rotation`)) (.pitch _returnvalue) (.yaw _returnvalue)) _animation_time_frame_2) false false))
                  (:`Finished`
                    (set `self.Finished?` true)
                    (`SceneComponent.SetWorldScale3D` _slimemonster_final2 (`KismetMathLibrary.VLerp` _returnvalue_5 (`KismetMathLibrary.MakeVector` (.x _returnvalue_5) (.y _returnvalue_5) (- (.z _returnvalue_5) (`self.scale`))) (`self.Alpha`)))
                    (goto _label)))
                (else
                  (goto _label_2 :!via `PlayFromStart`))))))))
    (:`then_2`
      (bind _outactors (`GameplayStatics.GetAllActorsOfClass` "/Game/mobs/TargetPoints/TP_4.TP_4_C"))
      (`|AIMoveTo` self (`self.K2_GetActorLocation` (`|GetArrayItem` _outactors)) :!label _label_3
        (:`OnSuccess`
          (bind _outactors_2 (`GameplayStatics.GetAllActorsOfClass` "/Game/mobs/TargetPoints/TP_3.TP_3_C"))
          (`|AIMoveTo` self (`self.K2_GetActorLocation` (`|GetArrayItem` _outactors_2))
            (:`OnSuccess`
              (goto _label_3))))))))

(event `self.Sphere.OnComponentBeginOverlap`
  (params (OverlappedComponent :type "PrimitiveComponent Object Reference") (OtherActor :type "Actor Object Reference") (OtherComp :type "PrimitiveComponent Object Reference") (OtherBodyIndex :type Integer) (bFromSweep :type Boolean) (SweepResult :type "HitResult Structure (by ref)"))
  (bind _charactermovement (`self.CharacterMovement`))
  ;[1 1 1] Health system
  (`|ExecutionSequence`
    (:`then_0`
      (cast `/Game/projectiles/FireBallProjctile` OtherActor)
      (bind _output_get (set `self.Health` (- (`self.Health`) 25.0)))
      (if (<= _output_get 0.0)
        (`GameplayStatics.SpawnEmitterAtLocation` "/Game/Particles/SlimeDeathEffect.SlimeDeathEffect" (`KismetMathLibrary.MakeVector` (.x (`self.K2_GetActorLocation`)) (.y (`self.K2_GetActorLocation`)) (+ (.z (`self.K2_GetActorLocation`)) 200.0)))
        (`self.K2_DestroyActor`)
        (else
          (`/Engine/EditorBlueprintResources/StandardMacros.DoOnce` false
            (:`Completed`
              (bind _asplayer_character (cast `/Game/CharacterStuff/PlayerCharacter` (`GameplayStatics.GetPlayerCharacter` 0)))
              (`|AIMoveTo` self (0.0 0.0 0.0) _asplayer_character) ; AI moves to player if gets hit
            )))))
    (:`then_1`
      ;[1 1 1] Later for attack animation (We use IsAttacking bool so we can stop the hoping animation and play the attack one)
      (cast `/Game/CharacterStuff/PlayerCharacter` OtherActor)
      (set `self.IsAttacking?` true) ; Later for attack animation
      (set `CharacterMovementComponent.MaxWalkSpeed` 0.0 _charactermovement)
      (`KismetSystemLibrary.Delay` 1.0) ; Cooldown time to let the player to get some distance
      (set `CharacterMovementComponent.MaxWalkSpeed` 650.0 _charactermovement)
      (set `self.IsAttacking?` false) ; Later for attack animation
    )))

(event `self.PawnSensing.OnSeePawn`
  (params (Pawn :type "Pawn Object Reference"))
  ;[1 1 1] Ai moves to player when sees him (Using pawn sensing)
  (bind _asplayer_character (cast `/Game/CharacterStuff/PlayerCharacter` Pawn))
  (`|AIMoveTo` self (0.0 0.0 0.0) _asplayer_character))

(fn `UserConstructionScript`)