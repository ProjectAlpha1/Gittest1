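; Enemy spawner actor that places slime and test monsters at its Box component's location when its Spawn event fires.
; For each of the two monster classes, it counts live actors in the world and spawns one AI pawn only while under a fixed cap.
; A sequence then starts a delay, after which the spawner destroys itself.
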(event `Spawn`
  (`|ExecutionSequence`
    (:`then_0`
      (bind _outactors (`GameplayStatics.GetAllActorsOfClass` "/Game/mobs/SlimeMonsterBP.SlimeMonsterBP_C"))
      (if (< (`KismetArrayLibrary.Array_Length` _outactors) 100)
        (`AIBlueprintHelperLibrary.SpawnAIFromClass` "/Game/mobs/SlimeMonsterBP.SlimeMonsterBP_C" null (`SceneComponent.K2_GetComponentLocation` (`self.Box`)))))
    (:`then_1`
      (bind _outactors_2 (`GameplayStatics.GetAllActorsOfClass` "/Game/mobs/MonsterTest.MonsterTest_C"))
      (if (< (`KismetArrayLibrary.Array_Length` _outactors_2) 100)
        (`AIBlueprintHelperLibrary.SpawnAIFromClass` "/Game/mobs/MonsterTest.MonsterTest_C" null (`SceneComponent.K2_GetComponentLocation` (`self.Box`)))))
    (:`then_2`
      (`KismetSystemLibrary.Delay` 30.0)
      (`self.K2_DestroyActor`))))

(fn `UserConstructionScript`)